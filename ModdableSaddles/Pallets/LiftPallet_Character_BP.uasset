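; Character Blueprint for a liftable pallet that can be carried, part of ModdableSaddles.
; Each tick it moves the mesh to a catchpole offset while carried and back to the origin otherwise.
; Unconnected graph logic would spawn a linked PalletCatchpole, attach two ropes to it and make the pallet follow it.
; The multi-use hooks are stubs, adding no entries and always reporting success.
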(event `self.ReceiveTick`
  (params (DeltaSeconds :type "Float (single-precision)"))
  (bind _mesh (`self.Mesh`))
  (if (`self.bIsCarried`)
    (`SceneComponent.SetRelativeLocation` _mesh (`self.CatchpoleOffset`) false)
    (else
      (`SceneComponent.SetRelativeLocation` _mesh (0.0 0.0 0.0) false))))

(fn `BPGetMultiUseEntries`
  (params (ForPC :type "PlayerController Object Reference") (MultiUseEntries :type "Array of Actor.MultiUseEntry Structure (by ref)"))
  (returns (ReturnValue :type "Array of Actor.MultiUseEntry Structure"))
  (return MultiUseEntries))

(fn `BPTryMultiUse`
  (params (ForPC :type "PlayerController Object Reference") (UseIndex :type Integer))
  (returns (ReturnValue :type Boolean))
  (return true))

(fn `UserConstructionScript`
  (`parent.UserConstructionScript`))